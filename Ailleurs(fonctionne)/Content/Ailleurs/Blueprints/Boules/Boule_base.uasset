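; Base glowing orb actor whose light, material and two particle effects share a set color and pulse with the music it plays.
; Unless DéplcementFluide is set, a looping random-delay impulse of force, scaled by the Centre's size, pulls the orb toward jittered points around Centre.
; PlayMusique crossfades two audio players while PlayCSV alternates two looping timelines, blending per-track CSV curves into the Intensité applied each Tick.
; StopMusique fades out both sound and intensity.
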(event `self.ReceiveTick`
  (params (DeltaSeconds :type "Float (single-precision)"))
  (bind _returnvalue (* (`self.Intensité`) 0.001))
  ;[1 1 1] Intensité
  (`|ExecutionSequence`
    (:`then_0`
      (`LightComponent.SetIntensity` (`self.PointLight`) (`self.Intensité`)))
    (:`then_1`
      (`MaterialInstanceDynamic.SetScalarParameterValue` (`self.mat_boule`) "int_mat" _returnvalue))
    (:`then_2`
      (`ParticleSystemComponent.SetFloatParameter` (`self.petites_lumières`) "Nb_part" (* _returnvalue 0.5)))
    (:`then_3`
      (`ParticleSystemComponent.SetFloatParameter` (`self.Aura_Lumière`) "Nb_part" _returnvalue))))

(event `self.ReceiveBeginPlay`
  (bind _amplitudexy (`self.AmplitudeXY`))
  (bind _amplitudez (`self.AmplitudeZ`))
  (bind _returnvalue (* _amplitudexy 0.5))
  ;[1 1 1] Boule suit le centre
  (if (not (`self.déplcement_fluide`))
    (`PrimitiveComponent.AddForce` (`self.boule`) (* (- (`KismetMathLibrary.MakeVector` (+ (.x (`SceneComponent.K2_GetComponentLocation` (`self.centre`))) (- (* (`KismetMathLibrary.RandomFloat`) _amplitudexy) _returnvalue)) (+ (.y (`SceneComponent.K2_GetComponentLocation` (`self.centre`))) (- (* (`KismetMathLibrary.RandomFloat`) _amplitudexy) _returnvalue)) (+ (.z (`SceneComponent.K2_GetComponentLocation` (`self.centre`))) (- (* (`KismetMathLibrary.RandomFloat`) _amplitudez) (* _amplitudez 0.5)))) (`SceneComponent.K2_GetComponentLocation` (`self.boule`))) (`self.Force`)) "None" false :!label _label)
    (`KismetSystemLibrary.Delay` (* (`self.Periode`) (+ (`KismetMathLibrary.RandomFloat`) 0.4)))
    (if true
      (goto _label))))

(event `PlayCSV`
  (params (NumMusique :type Integer) (Duration :type "Float (double-precision)"))
  (bind _musiquea (`self.musiqueA`))
  (bind _musiqueb (`self.musiqueB`))
  ;[1 1 1] CSV
  (`|ExecutionSequence`
    (:`then_0`
      (bind _isa (`/Engine/EditorBlueprintResources/StandardMacros.FlipFlop`)
        (:`A`
          (set `self.musiqueA` NumMusique)
          (`|ExecutionSequence` :!label _label_2
            (:`then_0`
              (bind (_direction _newtrack_0) (`Timeline|Timeline_1` :!via `PlayFromStart` :!label _label_3)
                (:`Update`
                  (set `self.Intensité` (* (`KismetMathLibrary.Lerp` (`CurveFloat.GetFloatValue` (`|GetArrayItem` (`self.CSV`) _musiquea) _newtrack_0) (`CurveFloat.GetFloatValue` (`|GetArrayItem` (`self.CSV`) _musiqueb) (stale _newtrack_0_2)) (`self.alpha`)) (`self.coef_intensité`)) :!label _label_4))))
            (:`then_1`
              (`KismetSystemLibrary.RetriggerableDelay` (`SoundBase.Duration` (`|GetArrayItem` (`self.Musiques`) _musiquea)))
              (goto _label_2))))
        (:`B`
          (set `self.musiqueB` NumMusique)
          (`|ExecutionSequence` :!label _label_5
            (:`then_0`
              (bind (_direction_2 _newtrack_0_2) (`Timeline|Timeline_2` :!via `PlayFromStart` :!label _label_6)
                (:`Update`
                  (goto _label_4))))
            (:`then_1`
              (`KismetSystemLibrary.RetriggerableDelay` (`SoundBase.Duration` (`|GetArrayItem` (`self.Musiques`) _musiqueb)))
              (goto _label_5))))))
    (:`then_1`
      (bind (_direction_3 _newtrack_0_3) (`Timeline|Timeline_3` :!via `PlayFromStart` :!label _label_7)
        (:`Update`
          (if _isa
            (bind _returnvalue (/ _newtrack_0_3 Duration))
            (set `self.alpha` (- 1.0 _returnvalue))
            (else
              (set `self.alpha` _returnvalue))))))
    (:`then_2`
      (`KismetSystemLibrary.Delay` Duration)
      (`|ExecutionSequence`
        (:`then_0`
          (goto _label_7 :!via `Stop`))
        (:`then_1`
          (if _isa
            (goto _label_6 :!via `Stop`)
            (else
              (goto _label_3 :!via `Stop`))))))
    (:`then_3`
      (set `self.coef_intensité` 1.0))))

(event `FadeOutCSV`
  (params (duration :type "Float (double-precision)"))
  ;[1 1 1] CSV
  (`|ExecutionSequence`
    (:`then_0`
      (bind (_direction _newtrack_0) (`Timeline|Timeline_0` :!via `PlayFromStart` :!label _label_8)
        (:`Update`
          (set `self.coef_intensité` (- 1.0 (/ _newtrack_0 duration))))))
    (:`then_1`
      (`KismetSystemLibrary.Delay` duration)
      (goto _label_8 :!via `Stop`))))

(fn `playMusique`
  (params (Num :type Integer) (Transition :type "Float (double-precision)"))
  (bind _musiqueplayer1 (`self.MusiquePlayer1`))
  (bind _musiqueplayer2 (`self.MusiquePlayer2`))
  (bind _output (`|GetArrayItem` (`self.Musiques`) Num))
  (if (`self.isUsingMP1`)
    (`AudioComponent.SetSound` _musiqueplayer2 _output)
    (`AudioComponent.FadeIn` _musiqueplayer2 Transition 1.0 0.0)
    (`AudioComponent.FadeOut` (`self.MusiquePlayer1`) Transition 0.0)
    (else
      (`AudioComponent.SetSound` _musiqueplayer1 _output)
      (`AudioComponent.FadeIn` _musiqueplayer1 Transition 1.0 0.0)
      (`AudioComponent.FadeOut` (`self.MusiquePlayer2`) Transition 0.0)))
  (set `self.isUsingMP1` (not (`self.isUsingMP1`)))
  (`self.PlayCSV` Num Transition))

(fn `setAmplXY`
  (params (NewAmplXY :type "Float (double-precision)"))
  (set `self.AmplitudeXY` NewAmplXY))

(fn `setAmplZ`
  (params (NewAmplZ :type "Float (double-precision)"))
  (set `self.AmplitudeZ` NewAmplZ))

(fn `setColor`
  (params (newColor :type "Color Structure"))
  (set `self.color` newColor)
  ;[1 1 1] set color
  (`|ExecutionSequence`
    (:`then_0`
      (bind _returnvalue (`PrimitiveComponent.CreateDynamicMaterialInstance` (`self.boule`) 0 "/Game/Ailleurs/Blueprints/Boules/M_Boule_base.M_Boule_base" "None"))
      (bind _output_get (set `self.mat_boule` _returnvalue))
      (`MaterialInstanceDynamic.SetVectorParameterValue` _output_get "Color" (`KismetMathLibrary.Conv_ColorToLinearColor` (`self.color`))))
    (:`then_1`
      (`ParticleSystemComponent.SetColorParameter` (`self.petites_lumières`) "Color" (`KismetMathLibrary.Conv_ColorToLinearColor` (`self.color`))))
    (:`then_2`
      (`ParticleSystemComponent.SetColorParameter` (`self.Aura_Lumière`) "Color" (`KismetMathLibrary.Conv_ColorToLinearColor` (`self.color`))))
    (:`then_3`
      (`LightComponent.SetLightColor` (`self.PointLight`) (`KismetMathLibrary.Conv_ColorToLinearColor` (`self.color`)) true))))

(fn `setMusiquesAndCSV`
  (params (musiques :type "Array of SoundWave Object Reference") (CSV :type "Array of CurveFloat Object Reference"))
  (set `self.Musiques` musiques)
  (set `self.CSV` CSV))

(fn `stopMusique`
  (params (FadeOutDuration :type "Float (double-precision)"))
  (`AudioComponent.FadeOut` (`self.MusiquePlayer1`) FadeOutDuration 0.0)
  (`AudioComponent.FadeOut` (`self.MusiquePlayer2`) FadeOutDuration 0.0)
  (`self.FadeOutCSV` FadeOutDuration))

(fn `UserConstructionScript`
  (`|ExecutionSequence`
    (:`then_0`
      ;[1 1 1] Adaptation de la 'force' à la masse
      (set `self.Force` (* 1700.0 (* (.x (`SceneComponent.K2_GetComponentScale` (`self.centre`))) (.y (`SceneComponent.K2_GetComponentScale` (`self.centre`)))))))
    (:`then_1`
      ;[1 1 1] set color
      (`|ExecutionSequence`
        (:`then_0`
          (bind _returnvalue (`PrimitiveComponent.CreateDynamicMaterialInstance` (`self.boule`) 0 "/Game/Ailleurs/Blueprints/Boules/M_Boule_base.M_Boule_base" "None"))
          (bind _output_get (set `self.mat_boule` _returnvalue))
          (`MaterialInstanceDynamic.SetVectorParameterValue` _output_get "Color" (`KismetMathLibrary.Conv_ColorToLinearColor` (`self.color`))))
        (:`then_1`
          (`ParticleSystemComponent.SetColorParameter` (`self.petites_lumières`) "Color" (`KismetMathLibrary.Conv_ColorToLinearColor` (`self.color`))))
        (:`then_2`
          (`ParticleSystemComponent.SetColorParameter` (`self.Aura_Lumière`) "Color" (`KismetMathLibrary.Conv_ColorToLinearColor` (`self.color`))))
        (:`then_3`
          (`LightComponent.SetLightColor` (`self.PointLight`) (`KismetMathLibrary.Conv_ColorToLinearColor` (`self.color`)) true))))))