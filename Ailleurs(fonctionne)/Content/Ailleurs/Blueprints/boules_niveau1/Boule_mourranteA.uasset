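; Glowing ball actor for level 1 ("Boule mourrante A") whose brightness follows a shared Material Parameter Collection value.
; Each tick it reads int_A and scales it into the point light intensity and the mesh material's int_mat parameter.
; On BeginPlay it polls a collection flag marking the end of loading, then enlarges PetitesLumieres and Traits and disables mesh gravity.
; The dynamic material instance setup is unconnected and never runs.
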(event `self.ReceiveTick`
  (params (DeltaSeconds :type "Float (single-precision)"))
  ;[1 1 1] intensité dynamique
  (bind _returnvalue (`KismetMaterialLibrary.GetScalarParameterValue` "/Game/Ailleurs/Autres/Boules_ParameterCollection1.Boules_ParameterCollection1" "int_A"))
  (`LightComponent.SetIntensity` (`self.PointLight`) (* _returnvalue 2.0))
  (`MeshComponent.SetScalarParameterValueOnMaterials` (`self.StaticMesh`) "int_mat" (* _returnvalue 0.008)))

(event `self.ReceiveBeginPlay`
  ;[1 1 1] fin chargement
  (bind _returnvalue (`KismetMaterialLibrary.GetScalarParameterValue` "/Game/Ailleurs/Autres/boolean_collection.boolean_collection" "boolean" :!label _label))
  (if (>= _returnvalue 0.5)
    (`SceneComponent.SetWorldScale3D` (`self.petites_lumieres`) (1.5 1.5 1.5))
    (`SceneComponent.SetWorldScale3D` (`self.traits`) (1.5 1.5 1.5))
    (`PrimitiveComponent.SetEnableGravity` (`self.StaticMesh`) false)
    (else
      (`KismetSystemLibrary.Delay` 0.1)
      (goto _label))))

(fn `UserConstructionScript`)