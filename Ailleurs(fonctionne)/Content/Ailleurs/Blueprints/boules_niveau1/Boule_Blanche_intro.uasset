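; Intro white ball actor ("Boule_Blanche_intro") for level 1, whose glow follows a shared intensity value.
; Each Tick reads the int_B scalar from Boules_ParameterCollection1 and scales it to drive the PointLight intensity and the mesh materials' int_mat parameter.
; The construction script is empty, with its dynamic material instance setup left disconnected.
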(event `self.ReceiveTick`
  (params (DeltaSeconds :type "Float (single-precision)"))
  ;[1 1 1] intensité dynamique
  (bind _returnvalue (`KismetMaterialLibrary.GetScalarParameterValue` "/Game/Ailleurs/Autres/Boules_ParameterCollection1.Boules_ParameterCollection1" "int_B"))
  (`LightComponent.SetIntensity` (`self.PointLight`) (* _returnvalue 2.0))
  (`MeshComponent.SetScalarParameterValueOnMaterials` (`self.StaticMesh`) "int_mat" (* _returnvalue 0.008)))

(fn `UserConstructionScript`)