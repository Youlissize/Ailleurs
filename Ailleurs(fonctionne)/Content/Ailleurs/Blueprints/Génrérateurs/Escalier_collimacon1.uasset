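; Spiral staircase step actor that recursively builds a temporary staircase at runtime, one step per actor.
; Shortly after BeginPlay, each step spawns the next at its Arrow transform and passes on a decremented NombreMarche until the count reaches zero.
; A Taille timeline animates the Marche component's non-uniform scale, while a delay destroys each step seconds later, so the staircase vanishes in spawn order.
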(event `self.ReceiveBeginPlay`
  (`KismetSystemLibrary.Delay` 0.1)
  (`|ExecutionSequence`
    (:`then_0`
      (`KismetSystemLibrary.Delay` 0.05)
      (if (not (== (`self.nombre_marche`) 0))
        (bind _returnvalue (`|SpawnActorFromClass` "Escalier_collimacon1_C" (`SceneComponent.K2_GetComponentToWorld` (`self.Arrow`)) "Undefined" "OverrideRootScale" null null))
        (bind _result (`/Engine/EditorBlueprintResources/StandardMacros.DecrementInt` (`self.nombre_marche`))
          (:`  `
            (set `/Game/Ailleurs/Blueprints/Génrérateurs/Escalier_collimacon1.nombre_marche` _result _returnvalue)))))
    (:`then_1`
      (`KismetSystemLibrary.Delay` 3.0)
      (`self.K2_DestroyActor`))
    (:`then_2`
      (bind (_direction _newtrack_0) (`Timeline|taille`)
        (:`Update`
          (`SceneComponent.SetRelativeScale3D` (`self.marche`) (`KismetMathLibrary.MakeVector` (* _newtrack_0 3.0) _newtrack_0 (* _newtrack_0 0.2))))))))

(fn `UserConstructionScript`)